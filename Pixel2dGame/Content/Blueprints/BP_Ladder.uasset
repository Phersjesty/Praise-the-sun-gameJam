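; BP_Ladder is a ladder actor that lets the player climb by holding W.
; Tick flags OnLadder when the player is within a narrow band on world X only, enabling input in both branches and printing debug text.
; Pressing W on the ladder switches the character to Flying and adds upward input, re-checking through a short Delay loop.
; Releasing W or leaving the band restores Walking at the next check.
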(event `self.ReceiveTick`
  (params (DeltaSeconds :type "Float (single-precision)"))
  (bind _returnvalue_x (`KismetMathLibrary.BreakVector` (`self.K2_GetActorLocation`)))
  (bind _returnvalue (`GameplayStatics.GetPlayerController` 0))
  (bind _returnvalue_x_2 (`KismetMathLibrary.BreakVector` (`self.K2_GetActorLocation` (`GameplayStatics.GetPlayerCharacter` 0))))
  (`|ExecutionSequence`
    (:`then_0`
      (set `self.DistanceLadder` (- _returnvalue_x _returnvalue_x_2)))
    (:`then_1`
      (`KismetSystemLibrary.PrintString` (`KismetStringLibrary.Conv_DoubleToString` (`self.DistanceLadder`))))
    (:`then_2`
      (if (`KismetMathLibrary.InRange_FloatFloat` (`self.DistanceLadder`) -10.0 10.0 false)
        (set `self.OnLadder` true)
        (`self.EnableInput` _returnvalue)
        (`KismetSystemLibrary.PrintString` "on")
        (else
          (set `self.OnLadder` false)
          (`self.EnableInput` _returnvalue)
          (`KismetSystemLibrary.PrintString` "off"))))))

(event `Key|W`
  (params (Key :type "Key Structure"))
  (bind _returnvalue (`GameplayStatics.GetPlayerPawn` 0))
  (:`Pressed`
    (if (`self.OnLadder`) :!label _label
      (if (`PlayerController.IsInputKeyDown` (`GameplayStatics.GetPlayerController` 0) "W")
        (`CharacterMovementComponent.SetMovementMode` (`Character.CharacterMovement` (`GameplayStatics.GetPlayerCharacter` 0)) "MOVE_Flying" 0)
        (`Pawn.AddMovementInput` _returnvalue (`self.GetActorUpVector` _returnvalue) 1.0 false)
        (`KismetSystemLibrary.Delay` 0.2)
        (goto _label)
        (else
          _)))
    (`CharacterMovementComponent.SetMovementMode` (`Character.CharacterMovement` (`GameplayStatics.GetPlayerCharacter` 0)) "MOVE_Walking" 0)))

(fn `UserConstructionScript`)