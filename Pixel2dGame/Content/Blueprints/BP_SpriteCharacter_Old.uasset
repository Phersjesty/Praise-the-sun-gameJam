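; BP_SpriteCharacter_Old is a character Blueprint, apparently an older sprite version, whose only logic here toggles the pause menu.
; The Pause Game input action creates the menu widget on first press and caches it in PauseMenuRef.
; Each press then adds or removes the menu, sets the game's paused state, and switches mouse cursor visibility and input mode between Game Only and Game and UI.
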(event `InputAction|Pause Game` :paused true
  (params (Key :type "Key Structure"))
  (bind _returnvalue (`GameplayStatics.GetPlayerController` 0))
  (bind _pausemenu_ref (`self.PauseMenu Ref`))
  ;[1 1 1] Pause/Unpause Game
  (:`Pressed`
    (`/Engine/EditorBlueprintResources/StandardMacros.IsValid` (`self.PauseMenu Ref`)
      (:`Is Valid`
        _)
      (:`Is Not Valid`
        (bind _returnvalue_2 (`|CreateWidget` "/Game/UI/PauseMenuWidget.PauseMenuWidget_C"))
        (set `self.PauseMenu Ref` _returnvalue_2)))
    (if (`GameplayStatics.IsGamePaused`)
      (`Widget.RemoveFromParent` _pausemenu_ref)
      (`GameplayStatics.SetGamePaused` false)
      (set `PlayerController.bShowMouseCursor` false _returnvalue)
      (`WidgetBlueprintLibrary.SetInputMode_GameOnly` _returnvalue)
      (else
        (`UserWidget.AddToViewport` _pausemenu_ref 0)
        (`GameplayStatics.SetGamePaused` true)
        (set `PlayerController.bShowMouseCursor` true _returnvalue)
        (`WidgetBlueprintLibrary.SetInputMode_GameAndUIEx` _returnvalue _pausemenu_ref "LockInFullscreen" false)))))

(fn `UserConstructionScript`)